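; Grenade projectile Blueprint that explodes on a short fixed timer after spawning.
; BeginPlay waits out a delay, then Explode spawns an explosion particle effect and applies full, non-falloff radial damage credited to the instigator's controller.
; It also draws a debug sphere showing the damage radius, then destroys itself.
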(event `self.ReceiveBeginPlay`
  (`KismetSystemLibrary.Delay` 1.0)
  (`self.Explode`))

(event `Explode`
  (bind _returnvalue (`self.K2_GetActorLocation`))
  (bind _damageradius (`self.DamageRadius`))
  (`GameplayStatics.SpawnEmitterAtLocation` "/Game/Weapons/WeaponEffects/Explosion/P_Explosion.P_Explosion" _returnvalue)
  (`GameplayStatics.ApplyRadialDamage` :`BaseDamage` 100.0 :`Origin` _returnvalue :`DamageRadius` _damageradius :`DamageCauser` self :`InstigatedByController` (`self.GetInstigatorController`) :`bDoFullDamage` true)
  (`KismetSystemLibrary.DrawDebugSphere` _returnvalue _damageradius 12 (struct :`R` 1.0 :`G` 0.657076 :`A` 1.0) 1.0 2.0)
  (`self.K2_DestroyActor`))

(fn `UserConstructionScript`)